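; BP_CarPlacer2 is a construction-time placer that scatters a handful of randomly chosen car meshes inside a box area.
; The Construction Script sizes the flat Box from BoxSize, then calls SpawnCar in a fixed loop.
; Each call adds a StaticMeshComponent with a random mesh, yaw and XY point from the box bounds.
; Subtracting actor location makes the point relative, targeting world Z zero and ignoring actor rotation and scale.
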(fn `SpawnCar`
  (bind _mesh (`self.mesh`))
  (bind (_origin _boxextent) (`KismetSystemLibrary.GetComponentBounds` (`self.Box`)))
  (bind (_returnvalue_x _returnvalue_y) (`KismetMathLibrary.BreakVector` (`KismetMathLibrary.RandomPointInBoundingBox` _origin _boxextent)))
  (bind _returnvalue (`AddComponent|NODE_AddStaticMeshComponent-0` :`RelativeTransform` (`KismetMathLibrary.MakeTransform` (- (`KismetMathLibrary.MakeVector` _returnvalue_x _returnvalue_y) (`self.K2_GetActorLocation`)) (`KismetMathLibrary.MakeRotator` 0.0 0.0 (`KismetMathLibrary.RandomFloatInRange` 0.0 360.0)))))
  (`StaticMeshComponent.SetStaticMesh` _returnvalue (`|GetArrayItem` _mesh (`KismetMathLibrary.RandomInteger` (`KismetArrayLibrary.Array_Length` _mesh)))))

(fn `UserConstructionScript`
  (`BoxComponent.SetBoxExtent` (`self.Box`) (`KismetMathLibrary.Conv_Vector2DToVector` (`self.Box Size`)) true)
  (for _ (range 6)
    (`self.SpawnCar`)))