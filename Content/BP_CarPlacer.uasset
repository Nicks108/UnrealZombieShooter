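; BP_CarPlacer is an actor that scatters car meshes at random within a flat box area.
; The construction script sizes the box from BoxSize with zero height, then assigns one random mesh from the Mesh array to an InstancedStaticMesh component.
; A fixed loop calls SpawnCar, which adds world-space instances at random points in the box bounds with random yaw.
; The layout rerolls whenever construction reruns, and no gameplay logic runs.
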(fn `Spawn Car`
  (params (Car :type "StaticMesh Object Reference"))
  (bind (_origin _boxextent) (`KismetSystemLibrary.GetComponentBounds` (`self.Box`)))
  (`InstancedStaticMeshComponent.AddInstance` (`self.InstancedStaticMesh`) (`KismetMathLibrary.MakeTransform` (`KismetMathLibrary.RandomPointInBoundingBox` _origin _boxextent) (`KismetMathLibrary.MakeRotator` 0.0 0.0 (`KismetMathLibrary.RandomFloatInRange` 0.0 360.0))) true))

(fn `UserConstructionScript`
  (bind _mesh (`self.mesh`))
  (`BoxComponent.SetBoxExtent` (`self.Box`) (`KismetMathLibrary.Conv_Vector2DToVector` (`self.Box Size`)) true)
  (`StaticMeshComponent.SetStaticMesh` (`self.InstancedStaticMesh`) (`|GetArrayItem` _mesh (`KismetMathLibrary.RandomInteger` (`KismetArrayLibrary.Array_Length` _mesh))))
  (for _ (range 6)
    (`self.Spawn Car` null)))