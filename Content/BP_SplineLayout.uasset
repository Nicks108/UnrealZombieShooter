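; BP_SplineLayout is a construction-script tool that lays a chosen mesh along a spline as a road, fence or row of props.
; Road mode adds one spline mesh per segment, bent to the point locations and tangents.
; Otherwise it fills an instanced static mesh at intervals of mesh X length plus an offset.
; Fence mode aims each instance at the next position; other instances keep zero rotation.
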(fn `GetLocationAtIndex`
  (params (A :type Integer))
  (returns (ReturnValue :type "Vector Structure"))
  (return (`SplineComponent.GetLocationAtDistanceAlongSpline` (`self.Spline`) (* A (`self.Spacing`)) "Local")))

(fn `MakeTransformForInstance`
  (params (InstanceIndex :type Integer) (IsFence :type Boolean))
  (returns (ReturnValue :type "Transform Structure"))
  (bind _returnvalue (`self.GetLocationAtIndex` InstanceIndex))
  (if IsFence
    (return (`KismetMathLibrary.MakeTransform` _returnvalue (`KismetMathLibrary.MakeRotFromX` (- (`self.GetLocationAtIndex` (+ InstanceIndex 1)) _returnvalue))))
    (else
      (return (`KismetMathLibrary.MakeTransform` (`self.GetLocationAtIndex` InstanceIndex))))))

(fn `UserConstructionScript`
  (locals (NumberOfInstances :type Integer :default 0))
  (bind _spline (`self.Spline`))
  (bind (_min _max) (break `Box` (`StaticMesh.GetBoundingBox` (`self.Mesh`))))
  (if (`self.IsRoad`)
    (for _index (range (+ (- (`SplineComponent.GetNumberOfSplinePoints` (`self.Spline`)) 2) 1))
      (bind _returnvalue (`AddComponent|NODE_AddSplineMeshComponent-0`))
      (`StaticMeshComponent.SetStaticMesh` _returnvalue (`self.Mesh`))
      (bind (_location _tangent) (`SplineComponent.GetLocationAndTangentAtSplinePoint` _spline _index "Local"))
      (bind (_location_2 _tangent_2) (`SplineComponent.GetLocationAndTangentAtSplinePoint` _spline (+ _index 1) "Local"))
      (`SplineMeshComponent.SetStartAndEnd` _returnvalue _location _tangent _location_2 _tangent_2 true)
      (`SceneComponent.K2_AttachToComponent` _returnvalue (`self.DefaultSceneRoot`) "None" "KeepRelative" "KeepRelative" "KeepRelative" true))
    (else
      (`StaticMeshComponent.SetStaticMesh` (`self.InstancedStaticMesh`) (`self.Mesh`))
      (bind _output_get (set `self.Spacing` (+ (.x (- _max _min)) (`self.Offset`))))
      (bind _output_get_2 (set `local.NumberOfInstances` (`KismetMathLibrary.FFloor` (/ (`SplineComponent.GetSplineLength` (`self.Spline`)) _output_get))))
      (for _index_2 (range (+ _output_get_2 1))
        (bind _returnvalue_2 (`self.MakeTransformForInstance` _index_2 (`self.IsFence`)))
        (`InstancedStaticMeshComponent.AddInstance` (`self.InstancedStaticMesh`) _returnvalue_2 false)))))